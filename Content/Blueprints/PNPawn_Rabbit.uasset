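; PNPawn_Rabbit is a pawn that deals damage on contact and watches for the player ahead of it.
; Each Tick, CanSeePlayerPawn casts a debug-drawn line trace along the actor's forward vector for SightLength and checks the hit actor for the "Player" tag, printing a message on a match.
; A capsule hit applies fixed damage to whatever actor it touches, with no filtering.
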(event OnComponentHit(CapsuleComponent)
  (params (HitComponent :type Primitive%20Component%20Object%20Reference) (OtherActor :type Actor%20Object%20Reference) (OtherComp :type Primitive%20Component%20Object%20Reference) (NormalImpulse :type Vector :default "0, 0, 0") (Hit :type Hit%20Result%20Structure%20%28by%20ref%29))
  (Game|Damage|ApplyDamage OtherActor 1e+02 0 0))

(event EventBeginPlay)

(event Collision|EventActorBeginOverlap
  (params (OtherActor :type Actor%20Object%20Reference)))

(event EventTick
  (params (DeltaSeconds :type Float%20%28single-precision%29))
  (if (AI|CanSeePlayerPawn)
    (Development|PrintString "See PNPlayerPawn!")))

(fn ConstructionScript)

(fn CanSeePlayerPawn
  (bind _returnvalue (Transformation|GetActorLocation))
  (bind _outhit (Collision|LineTraceByChannel _returnvalue (+ _returnvalue (* (Transformation|GetActorForwardVector) (Variables|Default|GetSightLength))) "TraceTypeQuery3" false 0 "ForOneFrame"))
  (return (Actor|ActorHasTag (.HitActor (Collision|BreakHitResult _outhit)) "Player")))