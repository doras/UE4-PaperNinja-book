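; PNPlayerPawn is the player character, with camera-relative movement, look, sprint and a coin count.
; Sprint switches max walk speed, while a looping timer drops a coin whenever flat speed reaches sprint speed.
; The first damage taken kills it: movement stops, the mesh ragdolls and a lifespan starts.
; ObtainScroll disables movement, flags the scroll as held and prints a goal message after a delay.
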(event Custom|ObtainScroll
  (Pawn|Components|CharacterMovement|DisableMovement (Variables|Character|GetCharacterMovement))
  (Variables|Default|SetHasScroll true)
  (Utilities|FlowControl|Delay 5.0)
  (Development|PrintString "Goal!!"))

(event EventBeginPlay
  (Variables|/Script/Engine.CharacterMovementComponent|SetMaxWalkSpeed (Variables|Character|GetCharacterMovement) (Variables|캐릭터|GetGroundWalkSpeed))
  (Utilities|Time|SetTimerbyFunctionName 0 "CheckSprintRisk" 0.5 true))

(event Collision|EventActorBeginOverlap
  (params (OtherActor :type Actor%20Object%20Reference)))

(event EventTick
  (params (DeltaSeconds :type Float%20%28single-precision%29)))

(event Game|Damage|EventAnyDamage
  (params (Damage :type Float%20%28single-precision%29) (DamageType :type Damage%20Type%20Object%20Reference) (InstigatedBy :type Controller%20Object%20Reference) (DamageCauser :type Actor%20Object%20Reference))
  (Utilities|FlowControl|DoOnce false
    (:Completed
      (Development|PrintString "Died!")
      (Pawn|Components|CharacterMovement|DisableMovement (Variables|Character|GetCharacterMovement))
      (Actor|SetLifeSpan 5.0)
      (Physics|SetSimulatePhysics (Variables|Character|GetMesh) true))))

(event Input|ActionEvents|InputActionSprint
  (params (Key :type Key%20Structure))
  (bind _charactermovement (Variables|Character|GetCharacterMovement))
  ;[1 1 1 0.2] Sprint 키 입력 시 속도 변경
  (:Pressed
    (Variables|/Script/Engine.CharacterMovementComponent|SetMaxWalkSpeed _charactermovement (Variables|Character|GetGroundSprintSpeed)) ; 스프린트 키/버튼을 눌렀을 때는 속도 증가
  )
  (:Released
    (Variables|/Script/Engine.CharacterMovementComponent|SetMaxWalkSpeed _charactermovement (Variables|캐릭터|GetGroundWalkSpeed)) ; 스프린트 키/버튼을 떼면 원래 속도로 복귀
  ))

(event Input|AxisEvents|InputAxisMoveForward
  (params (AxisValue :type Float%20%28single-precision%29))
  ;[1 1 1 0.2] 현재 카메라 방향 앞으로 이동
  (Pawn|Input|AddMovementInput (CallFunction|FlattenDirection (Math|Vector|GetForwardVector (Variables|Default|GetCamera))) AxisValue false) ; 앞으로 이동
)

(event Input|AxisEvents|InputAxisMoveRight
  (params (AxisValue :type Float%20%28single-precision%29))
  ;[1 1 1 0.2] 현재 카메라 방향 오른쪽으로 이동
  (Pawn|Input|AddMovementInput (CallFunction|FlattenDirection (Math|Vector|GetRightVector (Variables|Default|GetCamera))) AxisValue false))

(event Input|AxisEvents|InputAxisLookUp
  (params (AxisValue :type Float%20%28single-precision%29))
  ;[1 1 1 0.2] 카메라 각도 제어
  (Pawn|Input|AddControllerPitchInput AxisValue))

(event Input|AxisEvents|InputAxisLookRight
  (params (AxisValue :type Float%20%28single-precision%29))
  ;[1 1 1 0.2] 카메라 각도 제어
  (Pawn|Input|AddControllerYawInput AxisValue))

(fn ConstructionScript)

(fn AddCoin
  (params (Num :type Integer))
  (Variables|Default|SetNumOfCoins (+ (Variables|Default|GetNumOfCoins) Num)))

(fn GetNumOfCoins
  (return (Variables|Default|GetNumOfCoins)))

(fn DropCoin
  (if (>= (Variables|Default|GetNumOfCoins) 1)
    (Variables|Default|SetNumOfCoins (- (Variables|Default|GetNumOfCoins) 1))))

(fn CheckSprintRisk
  (if (>= (Utilities|GetFlatSpeed) (Variables|Character|GetGroundSprintSpeed)) ; 스프린트 속도가 되면
    (CallFunction|DropCoin) ; 코인을 감소시킵니다.
  ))